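; Game mode Blueprint that spawns an AI from a random spawner in the level when play begins.
; SpawnAI shuffles the BP_AISpawner actors and calls each one's SpawnAI until one succeeds, then prints a debug message and stops.
; The spawner list comes from LazyGetAISpawners, which finds the actors on first use and caches them behind a SpawnersFound flag.
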(event EventBeginPlay
  (CallFunction|SpawnAI))

(event EventTick
  (params (DeltaSeconds :type Float%20%28single-precision%29)))

(fn ConstructionScript)

(fn LazyGetAISpawners
  (Utilities|FlowControl|Sequence
    (:then_0
      (if (not (Variables|Default|GetSpawnersFound))
        (bind _outactors (Actor|GetAllActorsOfClass "/Game/BP_AISpawner.BP_AISpawner_C"))
        (Variables|Default|SetOutActors _outactors)
        (Variables|Default|SetSpawnersFound true)))
    (:then_1
      (return (Variables|Default|GetOutActors)))))

(fn SpawnAI
  (bind _outactors (CallFunction|LazyGetAISpawners))
  (bind _output_get (Variables|Default|SetLSpawners _outactors))
  (Utilities|Array|Shuffle _output_get)
  (bind _array_element (Utilities|Array|ForEachLoopwithBreak _output_get :!label _label)
    (:LoopBody
      (bind _result (Default|SpawnAI _array_element))
      (if _result
        (Development|PrintString "SPAWN" true true "(R=0.000000,G=0.660000,B=1.000000,A=1.000000)" 1e+01)
        (goto _label Break)))
    (:Completed
      (return))))