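; BP_AISpawner is an actor that spawns a ThirdPersonCharacter at its own location, with zero rotation and unit scale.
; BeginPlay makes a single call to SpawnAI, which runs only with authority and only once time since creation exceeds the last spawn time plus a cooldown.
; A valid spawn records the time; the function returns true for any spawn attempt, even a failed one, and false otherwise.
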(event EventBeginPlay
  (CallFunction|SpawnAI))

(event Collision|EventActorBeginOverlap
  (params (OtherActor :type Actor%20Object%20Reference)))

(event EventTick
  (params (DeltaSeconds :type Float%20%28single-precision%29)))

(fn ConstructionScript)

(fn SpawnAI
  (Networking|SwitchHasAuthority
    (:Authority
      (if (> (Actor|GetGameTimeSinceCreation) (+ (Variables|Default|GetLastTimeSpawned) (Variables|Default|GetSpawnCooldown)))
        (bind _returnvalue (Game|SpawnActorfromClass "/Game/ThirdPersonBP/Blueprints/ThirdPersonCharacter.ThirdPersonCharacter_C" (Math|Transform|MakeTransform (Transformation|GetActorLocation)) "Undefined" 0 0))
        (Utilities|IsValid _returnvalue
          (:Is%20Valid
            (Variables|Default|SetLastTimeSpawned (Actor|GetGameTimeSinceCreation))
            (return true))
          (:Is%20Not%20Valid
            (return true)))
        (else
          (return false))))
    (:Remote
      (return false))))